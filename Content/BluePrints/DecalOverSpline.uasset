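; DecalOverSpline is a spline-placed actor that builds a strip of spline mesh segments with a snow footprint tray material along its path.
; The construction script divides the spline length by the decal component's X size and adds one collision-enabled segment per step.
; Each segment follows local spline positions and tangents, with tangents clamped to segment length to limit distortion.
; Event graph events are disabled, so there is no runtime logic.
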(fn `UserConstructionScript`
  (bind _spline (`self.Spline`))
  (bind _spline_2 (`self.Spline`))
  (bind _decalsize_x (`KismetMathLibrary.BreakVector` (`DecalComponent.DecalSize` (`self.Mesh`))))
  (bind _output_get (set `self.xlength` _decalsize_x))
  (for _index (range (+ (`KismetMathLibrary.FTrunc` (/ (`SplineComponent.GetSplineLength` (`self.Spline`)) _output_get)) 1))
    (bind _returnvalue (`AddComponent|NODE_AddSplineMeshComponent-0`))
    (`PrimitiveComponent.SetCollisionEnabled` _returnvalue "QueryAndPhysics")
    (`SplineMeshComponent.SetForwardAxis` _returnvalue "X" true)
    (`PrimitiveComponent.CreateDynamicMaterialInstance` _returnvalue 0 "/Game/01_More_assets/footprint03_snow_tray_Inst.footprint03_snow_tray_Inst" "None")
    (bind _returnvalue_2 (* _index (`self.xlength`)))
    (bind _returnvalue_3 (* (+ _index 1) (`self.xlength`)))
    (`SplineMeshComponent.SetStartAndEnd` _returnvalue (`SplineComponent.GetLocationAtDistanceAlongSpline` _spline_2 _returnvalue_2 "Local") (`KismetMathLibrary.ClampVectorSize` (`SplineComponent.GetTangentAtDistanceAlongSpline` _spline_2 _returnvalue_2 "Local") 0.0 (`self.xlength`)) (`SplineComponent.GetLocationAtDistanceAlongSpline` _spline _returnvalue_3 "Local") (`KismetMathLibrary.ClampVectorSize` (`SplineComponent.GetTangentAtDistanceAlongSpline` _spline _returnvalue_3 "Local") 0.0 (`self.xlength`)) true)))